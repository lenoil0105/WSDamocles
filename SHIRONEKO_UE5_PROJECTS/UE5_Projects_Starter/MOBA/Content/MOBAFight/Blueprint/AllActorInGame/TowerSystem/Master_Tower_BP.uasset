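; Base MOBA tower that auto-fires at enemy creeps and characters and ends the match when destroyed.
; Tick refreshes every tower's HP widget and sphere-traces for opposing-team pawns, spawning a targeted Bullet_BP through a server event with a cooldown.
; Damage shows popup text; at zero HP a multicast fractures the destructible mesh.
; The server then halts players and creeps and sends each controller a titled kill scoreboard.
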(event Custom|Server:ShootBall
  ;[1 0.2936 0.02122] Tower Shoot Ball
  (Game|SpawnActorfromClass "/Game/MOBAFight/Blueprint/AllActorInGame/TowerSystem/Bullet_BP.Bullet_BP_C" (Math|Transform|MakeTransform (Transformation|GetActorLocation) (Math|Rotator|FindLookatRotation (Transformation|GetActorLocation) (Transformation|GetActorLocation (Variables|Default|GetActorTarget))) "1,1,1") "Undefined" 0 (Variables|Default|GetActorTarget) self 0)
  (Utilities|FlowControl|Delay 2.0)
  (Variables|Default|SetDisableTrigger false))

(event Custom|UpdateHP
  ;[0.07099 1 0.07567] Update HP
  (bind _outactors (Actor|GetAllActorsOfClass "Master_Tower_BP_C"))
  (for _array_element _outactors
    (bind _ashud_wb (Utilities|Casting|CastToHUD_WB (UserInterface|GetUserWidgetObject (Variables|Master_Tower_BP_C|GetHUD _array_element))))
    (Variables|/Game/MOBAFight/UI/NetworkGamePlay/HUD_WB.HUD_WB_C|SetHP _ashud_wb (Variables|Master_Tower_BP_C|GetHP _array_element))
    (Variables|/Game/MOBAFight/UI/NetworkGamePlay/HUD_WB.HUD_WB_C|SetMaxHP _ashud_wb (Variables|Master_Tower_BP_C|GetMaxHP _array_element))))

(event Custom|Server%20:%20EndGame
  ;[0.3589 0.3698 0.3616] Set Server End Game , Stop Movment All Actor , And Disable Input
  (bind _asnetwork_game_mode_bp (Utilities|Casting|CastToNetworkGameMode_BP (Game|GetGameMode)))
  (for _array_element (Variables|/Game/MOBAFight/Blueprint/NetworkGamePlay/NetworkGameMode_BP.NetworkGameMode_BP_C|GetAllPlayerController _asnetwork_game_mode_bp)
    (bind _asclient_side_controller_bp (Utilities|Casting|CastToClientSide_Controller_BP _array_element))
    ;;[1 1 1] for disable click acttive skill
    (Default|ServerEndGame _asclient_side_controller_bp)
    ;;[1 1 1] for disable click Movment
    (Default|Client:SetEndGame _asclient_side_controller_bp)
    (Components|Movement|StopMovementImmediately (Variables|/Script/Engine.Character|GetCharacterMovement (Variables|/Game/MOBAFight/Blueprint/NetworkGamePlay/ClientSide_Controller_BP.ClientSide_Controller_BP_C|GetServerSideCharacterRef _asclient_side_controller_bp))))
  (bind _outactors (Actor|GetAllActorsOfClass "/Game/MOBAFight/Blueprint/AllActorInGame/CreepSystem/Master_Creep_BP.Master_Creep_BP_C"))
  (for _array_element_2 _outactors
    ;;[1 1 1] Stop Creep Moving
    (Variables|/Game/MOBAFight/Blueprint/AllActorInGame/CreepSystem/Master_Creep_BP.Master_Creep_BP_C|SetEndGame? _array_element_2 true)
    (Components|Movement|StopMovementImmediately (Variables|/Script/Engine.Character|GetCharacterMovement _array_element_2)))
  ;;[1 1 1] Endgame and Show Score
  (CallFunction|AllPlayerShowScore))

(event Custom|AllPlayerShowScore
  ;[0.3589 0.3698 0.3616] Process All Player Show Score whne End Game
  (Utilities|Array|Clear (Variables|Default|GetEndScore))
  (bind _asnetwork_game_mode_bp (Utilities|Casting|CastToNetworkGameMode_BP (Game|GetGameMode)))
  (for _array_element (Variables|/Game/MOBAFight/Blueprint/NetworkGamePlay/NetworkGameMode_BP.NetworkGameMode_BP_C|GetAllPlayerController _asnetwork_game_mode_bp)
    (bind _asclient_side_controller_bp (Utilities|Casting|CastToClientSide_Controller_BP _array_element))
    (bind _title (CallFunction|FunctionTitle (Variables|/Game/MOBAFight/Blueprint/AllActorInGame/CharacterSystem/Master_Character_BP.Master_Character_BP_C|GetScoreKill (Variables|/Game/MOBAFight/Blueprint/NetworkGamePlay/ClientSide_Controller_BP.ClientSide_Controller_BP_C|GetServerSideCharacterRef _asclient_side_controller_bp))))
    (Utilities|Array|Add (Variables|Default|GetEndScore) (Utilities|Text|FormatText "{Name}         Kill  [{Score}]           {Title}" (.MyPlayerName (Utilities|Struct|BreakST_PlayerInfo (Variables|/Game/MOBAFight/Blueprint/NetworkGamePlay/ClientSide_Controller_BP.ClientSide_Controller_BP_C|GetPlayerInfoRef _asclient_side_controller_bp))) (Variables|/Game/MOBAFight/Blueprint/AllActorInGame/CharacterSystem/Master_Character_BP.Master_Character_BP_C|GetScoreKill (Variables|/Game/MOBAFight/Blueprint/NetworkGamePlay/ClientSide_Controller_BP.ClientSide_Controller_BP_C|GetServerSideCharacterRef _asclient_side_controller_bp)) _title)))
  (for _array_element_2 (Variables|/Game/MOBAFight/Blueprint/NetworkGamePlay/NetworkGameMode_BP.NetworkGameMode_BP_C|GetAllPlayerController _asnetwork_game_mode_bp)
    (bind _asclient_side_controller_bp_2 (Utilities|Casting|CastToClientSide_Controller_BP _array_element_2))
    (Default|SetScoreShow _asclient_side_controller_bp_2 (Variables|Default|GetEndScore))))

(event Custom|Multi:DestroyTower
  ;[1 0.4089 0.0831] Multi : Destroy Tower
  (Class|DestructibleComponent|ApplyRadiusDamage (Variables|Default|GetDestructibleComponent) 1e+01 (Transformation|GetActorLocation) 1e+02 2e+03 false)
  (Collision|SetCollisionEnabled (Variables|Default|GetBox) "NoCollision")
  (Utilities|FlowControl|Delay 4.0)
  (Actor|DestroyActor))

(event Custom|ShowBoxText
  (params (TextInput :type Text))
  ;[0.3589 0.3698 0.3616] Show Text Box Message
  (bind _asbox_text_wb (Utilities|Casting|CastToBoxText_WB (UserInterface|GetUserWidgetObject (Variables|Default|GetBoxText))))
  (Variables|/Game/MOBAFight/UI/NetworkGamePlay/BoxText_WB.BoxText_WB_C|SetText _asbox_text_wb TextInput)
  (UserInterface|Animation|PlayAnimation _asbox_text_wb (Variables|/Game/MOBAFight/UI/NetworkGamePlay/BoxText_WB.BoxText_WB_C|GetShowBox _asbox_text_wb) 0.0 1 "Forward" 1.0 false))

(event EventTick
  (params (DeltaSeconds :type Float%20%28single-precision%29))
  ;[0.02924 1 0.08066] Tower Tigger Detect Enemy
  (Utilities|FlowControl|Sequence
    (:then_0
      (CallFunction|UpdateHP))
    (:then_1
      (if (not (Variables|Default|GetDestroyTower))
        (if (not (Variables|Default|GetDisableTrigger))
          (bind _outhits (Collision|MultiSphereTraceForObjects (Transformation|GetActorLocation) (+ (Transformation|GetActorLocation) (Math|Vector|RotateVector "1.000000, 0,0.000000" (Transformation|GetActorRotation))) 5e+02 (Utilities|Array|MakeArray "ObjectTypeQuery3") false 0 "None" true "(R=1.000000,G=0.553293,B=0.000000,A=1.000000)"))
          (bind _array_element (Utilities|Array|ForEachLoopwithBreak _outhits :!label _label)
            (:LoopBody
              (bind _asmaster_creep_bp (Utilities|Casting|CastToMaster_Creep_BP (.HitActor (Collision|BreakHitResult _array_element)))
                (:then
                  (if (!= (Variables|/Game/MOBAFight/Blueprint/AllActorInGame/CreepSystem/Master_Creep_BP.Master_Creep_BP_C|GetTeam _asmaster_creep_bp) (Variables|Default|GetTeam))
                    (Variables|Default|SetActorTarget _asmaster_creep_bp)
                    (if (not (Variables|/Game/MOBAFight/Blueprint/AllActorInGame/CreepSystem/Master_Creep_BP.Master_Creep_BP_C|GetDie? _asmaster_creep_bp))
                      (Variables|Default|SetDisableTrigger true :!label _label_2)
                      (CallFunction|Server:ShootBall)
                      (goto _label Break))))
                (:CastFailed
                  (bind _asmaster_character_bp (Utilities|Casting|CastToMaster_Character_BP (.HitActor (Collision|BreakHitResult _array_element))))
                  (if (!= (Variables|/Game/MOBAFight/Blueprint/AllActorInGame/CharacterSystem/Master_Character_BP.Master_Character_BP_C|GetTeam _asmaster_character_bp) (Variables|Default|GetTeam))
                    (Variables|Default|SetActorTarget _asmaster_character_bp)
                    (if (not (Variables|/Game/MOBAFight/Blueprint/AllActorInGame/CharacterSystem/Master_Character_BP.Master_Character_BP_C|GetDie? _asmaster_character_bp))
                      (goto _label_2))))))))))))

(event Game|Damage|EventAnyDamage
  (params (Damage :type Float%20%28single-precision%29) (DamageType :type Damage%20Type%20Object%20Reference) (InstigatedBy :type Controller%20Object%20Reference) (DamageCauser :type Actor%20Object%20Reference))
  ;[1 0.2936 0.02122] Event Take Damage
  (CallFunction|ShowBoxText (Utilities|Text|FormatText "Get Damage -{Number}" Damage))
  (Variables|Default|SetHP (- (Variables|Default|GetHP) Damage))
  (if (<= (Variables|Default|GetHP) 0.0)
    (if (not (Variables|Default|GetDestroyTower))
      (Variables|Default|SetDestroyTower true)
      (CallFunction|Multi:DestroyTower)
      (CallFunction|Server:EndGame))))

(event MouseInput|EventActorBeginCursorOver
  (bind _destructiblecomponent (Variables|Default|GetDestructibleComponent))
  ;[1 1 1] Hightlight Mouse Over Object
  (Rendering|SetRenderCustomDepth _destructiblecomponent true)
  ;;[1 1 1] Setup Green Custom Colour
  (Rendering|SetCustomDepthStencilValue _destructiblecomponent 2))

(event MouseInput|EventActorEndCursorOver
  ;[1 1 1] Hightlight Mouse Over Object
  (Rendering|SetRenderCustomDepth (Variables|Default|GetDestructibleComponent) false))

(event Collision|EventActorBeginOverlap
  (params (OtherActor :type Actor%20Object%20Reference)))

(fn ConstructionScript)

(fn FunctionTitle
  (params (NumKill :type Integer))
  (if (<= NumKill 1)
    (LocalVariables|SetLocalTitle "Nooby")
    (elif (<= NumKill 3)
      (LocalVariables|SetLocalTitle "Normal")
      (else
        (LocalVariables|SetLocalTitle "God"))))
  (return (Utilities|Text|FormatText "Title  = {Title}" (LocalVariables|GetLocalTitle))))