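; Tower projectile for the MOBA tower system that damages one assigned target actor.
; On BeginPlay it copies Damage from its owning Master_Tower_BP, then destroys itself after a short delay as a lifetime limit.
; When its sphere begins overlapping the target, it destroys itself and applies that damage with the owner as damage causer, ignoring all other actors.
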(event OnComponentBeginOverlap(Sphere1)
  (params (OverlappedComponent :type Primitive%20Component%20Object%20Reference) (OtherActor :type Actor%20Object%20Reference) (OtherComp :type Primitive%20Component%20Object%20Reference) (OtherBodyIndex :type Integer) (bFromSweep :type Boolean) (SweepResult :type Hit%20Result%20Structure%20%28by%20ref%29))
  (if (== OtherActor (Variables|Default|GetActorTarget))
    (Actor|DestroyActor)
    (Game|Damage|ApplyDamage (Variables|Default|GetActorTarget) (Variables|Default|GetDamage) 0 (Variables|Default|GetOwnerBullet))))

(event EventBeginPlay
  (bind _asmaster_tower_bp (Utilities|Casting|CastToMaster_Tower_BP (Variables|Default|GetOwnerBullet))
    (:then
      (Variables|Default|SetDamage (Variables|/Game/MOBAFight/Blueprint/AllActorInGame/TowerSystem/Master_Tower_BP.Master_Tower_BP_C|GetDamage _asmaster_tower_bp)))
    (:CastFailed
      _))
  (Utilities|FlowControl|Delay 1.5)
  (Actor|DestroyActor))

(fn ConstructionScript)