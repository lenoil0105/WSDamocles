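; Base MOBA lane creep that walks to its team's target point via AI MoveTo and destroys itself on arrival.
; Tick refreshes every creep's HP widget and sphere-traces for enemy creeps, towers or characters.
; A found target halts it for an attack montage, with damage applied through DamageBPINF, then it rescans.
; Death credits a character killer, pushes team scores to clients through a server event, and grants EXP to all living opposing characters.
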(event Custom|UpdateKillScore
  (params (ActorKiller :type Actor%20Object%20Reference))
  (bind _asmaster_character_bp (Utilities|Casting|CastToMaster_Character_BP ActorKiller))
  (Variables|/Game/MOBAFight/Blueprint/AllActorInGame/CharacterSystem/Master_Character_BP.Master_Character_BP_C|SetScoreKill _asmaster_character_bp (+ (Variables|/Game/MOBAFight/Blueprint/AllActorInGame/CharacterSystem/Master_Character_BP.Master_Character_BP_C|GetScoreKill _asmaster_character_bp) 1)))

(event Custom|CreepMoveLocation
  ;[0.151 0.151 0.151] Creep Move to Goal
  (if (== (Variables|Attribute|GetTeam) 1)
    (Variables|Default|SetTargetPointMove (Variables|Default|GetTargetPoint2))
    (else
      (Variables|Default|SetTargetPointMove (Variables|Default|GetTargetPoint1))))
  (Utilities|FlowControl|Delay 0.2)
  (AI|AIMoveTo self (Transformation|GetActorLocation (Variables|Default|GetTargetPointMove)) 0 5.0 false
    (:then
      (Variables|Default|SetDisableEventTickFlag false))
    (:OnSuccess
      (Variables|Default|SetFinishGoal true)
      (Variables|Default|SetDisableEventTickFlag true)
      (Utilities|FlowControl|Delay 0.2)
      (Actor|DestroyActor))))

(event Custom|SearchEnemyActor
  ;[0.151 0.151 0.151] Creep Scan Enemy  , Attack Animetion  And Damage Event
  (if (and (not (Variables|Default|GetEndGame?)) (not (Variables|Default|GetDie?)))
    (Utilities|IsValid (Variables|Attribute|GetEnemyActor)
      (:Is%20Not%20Valid
        (bind _outhits (Collision|MultiSphereTraceForObjects (Transformation|GetActorLocation) (+ (Transformation|GetActorLocation) (Math|Vector|RotateVector "1.000000, 0,0.000000" (Transformation|GetActorRotation))) 3e+02 (Utilities|Array|MakeArray "ObjectTypeQuery3" "ObjectTypeQuery6") false 0 "None"))
        (bind _array_element (Utilities|Array|ForEachLoopwithBreak _outhits :!label _label)
          (:LoopBody
            (bind _asmaster_creep_bp (Utilities|Casting|CastToMaster_Creep_BP (.HitActor (Collision|BreakHitResult _array_element)))
              (:then
                (if (and (!= (Variables|Master_Creep_BP_C|GetTeam _asmaster_creep_bp) (Variables|Attribute|GetTeam)) (> (Variables|Master_Creep_BP_C|GetHP _asmaster_creep_bp) 0.0))
                  (Variables|Attribute|SetEnemyActor _asmaster_creep_bp)
                  (goto _label Break)))
              (:CastFailed
                (bind _asmaster_tower_bp (Utilities|Casting|CastToMaster_Tower_BP (.HitActor (Collision|BreakHitResult _array_element)))
                  (:then
                    (if (and (!= (Variables|/Game/MOBAFight/Blueprint/AllActorInGame/TowerSystem/Master_Tower_BP.Master_Tower_BP_C|GetTeam _asmaster_tower_bp) (Variables|Attribute|GetTeam)) (> (Variables|/Game/MOBAFight/Blueprint/AllActorInGame/TowerSystem/Master_Tower_BP.Master_Tower_BP_C|GetHP _asmaster_tower_bp) 0.0))
                      (Variables|Attribute|SetEnemyActor _asmaster_tower_bp)
                      (goto _label Break)))
                  (:CastFailed
                    (bind _asmaster_character_bp (Utilities|Casting|CastToMaster_Character_BP (.HitActor (Collision|BreakHitResult _array_element))))
                    (if (and (!= (Variables|/Game/MOBAFight/Blueprint/AllActorInGame/CharacterSystem/Master_Character_BP.Master_Character_BP_C|GetTeam _asmaster_character_bp) (Variables|Attribute|GetTeam)) (> (Variables|/Game/MOBAFight/Blueprint/AllActorInGame/CharacterSystem/Master_Character_BP.Master_Character_BP_C|GetHP _asmaster_character_bp) 0.0))
                      (Variables|Attribute|SetEnemyActor _asmaster_character_bp)
                      (goto _label Break)))))))
          (:Completed
            (Utilities|IsValid (Variables|Attribute|GetEnemyActor)
              (:Is%20Valid
                (Variables|Default|SetDisableEventTickFlag true)
                (CallFunction|MovetoAttack (Variables|Attribute|GetEnemyActor)))
              (:Is%20Not%20Valid
                (if (Variables|Default|GetDisableEventTickFlag)
                  (Variables|Default|SetDisableEventTickFlag false)
                  (CallFunction|CreepMoveLocation))))))))))

(event Custom|Server%20:%20AddScore
  (params (DamageCauser :type Actor%20Object%20Reference))
  (bind _gameinstanceref (Variables|Default|GetGameInstanceRef))
  ;[0.02924 1 0.08066] Update Score When Die Only Character Kill
  (bind _asmaster_character_bp (Utilities|Casting|CastToMaster_Character_BP DamageCauser))
  (if (!= (Variables|/Game/MOBAFight/Blueprint/AllActorInGame/CharacterSystem/Master_Character_BP.Master_Character_BP_C|GetTeam _asmaster_character_bp) (Variables|Attribute|GetTeam))
    (switch int (Variables|/Game/MOBAFight/Blueprint/AllActorInGame/CharacterSystem/Master_Character_BP.Master_Character_BP_C|GetTeam _asmaster_character_bp)
      (:1
        (Variables|/Game/MOBAFight/Blueprint/AllLevel/MasterGameInstance_BP.MasterGameInstance_BP_C|SetScoreAlpha _gameinstanceref (+ (Variables|/Game/MOBAFight/Blueprint/AllLevel/MasterGameInstance_BP.MasterGameInstance_BP_C|GetScoreAlpha _gameinstanceref) 1)))
      (:2
        (Variables|/Game/MOBAFight/Blueprint/AllLevel/MasterGameInstance_BP.MasterGameInstance_BP_C|SetScoreBeta _gameinstanceref (+ (Variables|/Game/MOBAFight/Blueprint/AllLevel/MasterGameInstance_BP.MasterGameInstance_BP_C|GetScoreBeta _gameinstanceref) 1))))
    (CallFunction|AllUpdateScore)))

(event Custom|AllUpdateScore
  ;[0.02924 1 0.08066] Update Score All Client
  (bind _asnetwork_game_mode_bp (Utilities|Casting|CastToNetworkGameMode_BP (Game|GetGameMode)))
  (for _array_element (Variables|/Game/MOBAFight/Blueprint/NetworkGamePlay/NetworkGameMode_BP.NetworkGameMode_BP_C|GetAllPlayerController _asnetwork_game_mode_bp)
    (bind _asclient_side_controller_bp (Utilities|Casting|CastToClientSide_Controller_BP _array_element))
    (Utilities|IsValid (Variables|/Game/MOBAFight/Blueprint/NetworkGamePlay/ClientSide_Controller_BP.ClientSide_Controller_BP_C|GetServerSideCharacterRef _asclient_side_controller_bp)
      (:Is%20Valid
        (Default|ClientUpDateScore _asclient_side_controller_bp (Variables|/Game/MOBAFight/Blueprint/AllLevel/MasterGameInstance_BP.MasterGameInstance_BP_C|GetScoreAlpha (Variables|/Game/MOBAFight/Blueprint/AllActorInGame/CharacterSystem/Master_Character_BP.Master_Character_BP_C|GetGameInstanceRef (Variables|/Game/MOBAFight/Blueprint/NetworkGamePlay/ClientSide_Controller_BP.ClientSide_Controller_BP_C|GetServerSideCharacterRef _asclient_side_controller_bp))) (Variables|/Game/MOBAFight/Blueprint/AllLevel/MasterGameInstance_BP.MasterGameInstance_BP_C|GetScoreBeta (Variables|/Game/MOBAFight/Blueprint/AllActorInGame/CharacterSystem/Master_Character_BP.Master_Character_BP_C|GetGameInstanceRef (Variables|/Game/MOBAFight/Blueprint/NetworkGamePlay/ClientSide_Controller_BP.ClientSide_Controller_BP_C|GetServerSideCharacterRef _asclient_side_controller_bp))))))))

(event Custom|DieAction
  ;[0.6615 0.05121 0.005115] Event Damage
  ;;[1 1 1] Stop Old Animation
  (Components|Animation|SetAnimationMode (Variables|Character|GetMesh) "AnimationBlueprint")
  (Components|Movement|StopMovementImmediately (Variables|Character|GetCharacterMovement))
  (Utilities|FlowControl|Delay 2.0)
  (Actor|DestroyActor))

(event Custom|UpdateHUD
  ;[0.04928 1 0.08844] Update HUD Creep All Time
  (bind _outactors (Actor|GetAllActorsOfClass "Master_Creep_BP_C"))
  (for _array_element _outactors
    (bind _ashud_wb (Utilities|Casting|CastToHUD_WB (UserInterface|GetUserWidgetObject (Variables|Master_Creep_BP_C|GetHUD _array_element))))
    (Variables|/Game/MOBAFight/UI/NetworkGamePlay/HUD_WB.HUD_WB_C|SetHP _ashud_wb (Variables|Master_Creep_BP_C|GetHP _array_element))
    (Variables|/Game/MOBAFight/UI/NetworkGamePlay/HUD_WB.HUD_WB_C|SetMaxHP _ashud_wb (Variables|Master_Creep_BP_C|GetMaxHP _array_element))))

(event Custom|AddEXPPlayer
  ;[1 0 0.8571] ** Update 4.00 ** Add EXP to Player
  (bind _outactors (Actor|GetAllActorsOfClass "/Game/MOBAFight/Blueprint/AllActorInGame/CharacterSystem/Master_Character_BP.Master_Character_BP_C"))
  (for _array_element _outactors
    (if (not (Variables|/Game/MOBAFight/Blueprint/AllActorInGame/CharacterSystem/Master_Character_BP.Master_Character_BP_C|GetDie? _array_element))
      (if (!= (Variables|/Game/MOBAFight/Blueprint/AllActorInGame/CharacterSystem/Master_Character_BP.Master_Character_BP_C|GetTeam _array_element) (Variables|Attribute|GetTeam))
        (Default|CallAddEXP _array_element (Variables|Attribute|GetEXP))))))

(event Custom|MovetoAttack
  (params (actor :type Actor%20Object%20Reference))
  (bind _returnvalue (Transformation|GetActorLocation))
  (bind _returnvalue_2 (Transformation|GetActorLocation actor))
  (bind _returnvalue_3 (Math|Rotator|FindLookatRotation _returnvalue _returnvalue_2))
  (bind (_roll _pitch _yaw) (Math|Rotator|BreakRotator _returnvalue_3))
  ;[0.151 0.151 0.151] Creep Scan Enemy  , Attack Animetion  And Damage Event
  (Variables|Attribute|SetEnemyActor actor)
  (Utilities|IsValid (Variables|Attribute|GetEnemyActor)
    (:Is%20Valid
      (Components|Movement|StopMovementImmediately (Variables|Character|GetCharacterMovement))
      (Transformation|SetActorRotation (Math|Rotator|MakeRotator _roll 0.0 _yaw))
      (Animation|PlayAnimMontage "/Game/MOBAFight/Mannequin/Animations/TwinSword_Attack13_Montage.TwinSword_Attack13_Montage" 1.0 "None")
      (Utilities|FlowControl|Delay 2.0)
      (Variables|Attribute|SetEnemyActor 0)
      (CallFunction|SearchEnemyActor))))

(event Custom|EventHitDamage
  ;[0.6615 0.05121 0.005115] Event Damage
  (Game|Damage|ApplyDamage (Variables|Attribute|GetEnemyActor) (Variables|Default|GetDamage) 0 self))

(event Custom|ShowBoxText
  (params (TextInput :type Text))
  ;[0.3589 0.3698 0.3616] Show Text Box Message
  (bind _asbox_text_wb (Utilities|Casting|CastToBoxText_WB (UserInterface|GetUserWidgetObject (Variables|Default|GetBoxText))))
  (Variables|/Game/MOBAFight/UI/NetworkGamePlay/BoxText_WB.BoxText_WB_C|SetText _asbox_text_wb TextInput)
  (UserInterface|Animation|PlayAnimation _asbox_text_wb (Variables|/Game/MOBAFight/UI/NetworkGamePlay/BoxText_WB.BoxText_WB_C|GetShowBox _asbox_text_wb) 0.0 1 "Forward" 1.0 false))

(event EventBeginPlay
  ;[0.151 0.151 0.151] Begin Action
  (bind _asmaster_game_instance_bp (Utilities|Casting|CastToMasterGameInstance_BP (Game|GetGameInstance)))
  (Variables|Default|SetGameInstanceRef _asmaster_game_instance_bp)
  (bind _outactors (Actor|GetAllActorsOfClass "/Game/MOBAFight/Blueprint/NetworkGamePlay/RuleWorld_BP.RuleWorld_BP_C"))
  (Variables|Default|SetTargetPoint1 (Variables|/Game/MOBAFight/Blueprint/NetworkGamePlay/RuleWorld_BP.RuleWorld_BP_C|GetTargetPoint1 (Utilities|Array|Get(acopy) _outactors)))
  (Variables|Default|SetTargetPoint2 (Variables|/Game/MOBAFight/Blueprint/NetworkGamePlay/RuleWorld_BP.RuleWorld_BP_C|GetTargetPoint2 (Utilities|Array|Get(acopy) _outactors)))
  (CallFunction|CreepMoveLocation))

(event Game|Damage|EventAnyDamage
  (params (Damage :type Float%20%28single-precision%29) (DamageType :type Damage%20Type%20Object%20Reference) (InstigatedBy :type Controller%20Object%20Reference) (DamageCauser :type Actor%20Object%20Reference))
  ;[0.6615 0.05121 0.005115] Event Damage
  (CallFunction|ShowBoxText (Utilities|Text|FormatText "Get Damage -{Number}" Damage))
  (if (not (Variables|Default|GetDie?))
    (Variables|Attribute|SetHP (- (Variables|Attribute|GetHP) Damage))
    (if (<= (Variables|Attribute|GetHP) 0.0)
      (Variables|Default|SetDie? true)
      (CallFunction|DieAction)
      (CallFunction|UpdateKillScore DamageCauser)
      (CallFunction|Server:AddScore DamageCauser)
      ;[1 0 0.8571] Version 4.00 Add EXP Player
      (CallFunction|AddEXPPlayer))))

(event EventDamageBPINF
  ;[0.151 0.151 0.151] Creep Scan Enemy  , Attack Animetion  And Damage Event
  (CallFunction|EventHitDamage))

(event EventTick
  (params (DeltaSeconds :type Float%20%28single-precision%29))
  ;[0.02924 1 0.08066] Event Tick
  (Utilities|FlowControl|Sequence
    (:then_0
      (CallFunction|UpdateHUD)
      (if (not (Variables|Default|GetDisableEventTickFlag))
        (CallFunction|SearchEnemyActor)))
    (:then_1
      (if (Variables|Default|GetEndGame?)
        ;;[1 1 1] Stop Old Animation
        (Components|Animation|SetAnimationMode (Variables|Character|GetMesh) "AnimationBlueprint")
        (Components|Movement|StopMovementImmediately (Variables|Character|GetCharacterMovement))))))

(event MouseInput|EventActorBeginCursorOver
  ;[0.02924 1 0.08066] HightLight Mouse Over
  (Rendering|SetRenderCustomDepth (Variables|Character|GetMesh) true))

(event MouseInput|EventActorEndCursorOver
  ;[0.02924 1 0.08066] HightLight Mouse Over
  (Rendering|SetRenderCustomDepth (Variables|Character|GetMesh) false))

(fn ConstructionScript)