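; Game instance Blueprint that manages front-end menus and multiplayer session hosting and joining for the MOBA game.
; A save-slot check opens the main menu for returning players, or the options menu with a welcome message on first run.
; Menu and loading screen widgets are created once, cached and re-added to the viewport.
; Hosting creates a session and opens LobbyMap as a listen server; hosting and joining both show the loading screen first.
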(event Custom|ShowOptionMenu
  ;[1 1 1] Show Option Menu
  (Utilities|IsValid (Variables|Widget|GetOptionMenuWB)
    (:Is%20Valid
      _)
    (:Is%20Not%20Valid
      (bind _returnvalue (UserInterface|CreateWidget "/Game/MOBAFight/UI/MainMenu/OptionsMenu_WB.OptionsMenu_WB_C"))
      (Variables|Widget|SetOptionMenuWB _returnvalue)))
  (UserInterface|Viewport|AddtoViewport (Variables|Widget|GetOptionMenuWB) 0)
  (if (not (Variables|NotsetValues|GetCreatedSaveFile?))
    (Variables|/Game/MOBAFight/UI/MainMenu/OptionsMenu_WB.OptionsMenu_WB_C|SetWelcomeMessageVis (Variables|Widget|GetOptionMenuWB) "Visible")))

(event Custom|ShowMainMenu
  (bind _returnvalue (Game|GetPlayerController 0))
  ;[1 1 1] Show Main Menu
  (Utilities|IsValid (Variables|Widget|GetMainMenuWB)
    (:Is%20Valid
      _)
    (:Is%20Not%20Valid
      (bind _returnvalue_2 (UserInterface|CreateWidget "/Game/MOBAFight/UI/MainMenu/MainMenu_WB.MainMenu_WB_C" _returnvalue))
      (Variables|Widget|SetMainMenuWB _returnvalue_2)))
  (UserInterface|Viewport|AddtoViewport (Variables|Widget|GetMainMenuWB) 0)
  (Variables|/Script/Engine.PlayerController|SetbShowMouseCursor _returnvalue true))

(event Custom|SaveGameCheck
  ;[1 1 1] Check for Save Game
  (bind _returnvalue (SaveGame|DoesSaveGameExist (Variables|NotsetValues|GetPlayerSettingSave)))
  (if _returnvalue
    (CallFunction|ShowMainMenu)
    (Variables|NotsetValues|SetCreatedSaveFile? true)
    (else
      (CallFunction|ShowOptionMenu)
      (Variables|/Script/Engine.PlayerController|SetbShowMouseCursor (Game|GetPlayerController 0) true))))

(event Custom|JoinServer
  (params (SessionToJoin :type Blueprint%20Session%20Result%20Structure))
  ;[1 1 1] Joint Game Sesion
  (CallFunction|ShowLoadingScreen)
  (|JoinSession (Game|GetPlayerController 0) SessionToJoin))

(event Custom|ShowLoadingScreen
  ;[1 1 1] Show Loading Screen
  (Utilities|IsValid (Variables|Widget|GetShowLoadingScreenWB)
    (:Is%20Valid
      _)
    (:Is%20Not%20Valid
      (bind _returnvalue (UserInterface|CreateWidget "/Game/MOBAFight/UI/LoadingScreen_WB.LoadingScreen_WB_C"))
      (Variables|Widget|SetShowLoadingScreenWB _returnvalue)))
  (UserInterface|Viewport|AddtoViewport (Variables|Widget|GetShowLoadingScreenWB) 0))

(event Custom|LuanchLobby
  ;[1 1 1] Keep EveryOne Go To Gameplay Map
  (CallFunction|ShowLoadingScreen)
  (|Session (Game|GetPlayerController 0) (Variables|Default|GetMaxPlayers) (Variables|Default|GetUserLAN)
    (:OnSuccess
      (Game|OpenLevel(byName) "LobbyMap" true "listen"))))