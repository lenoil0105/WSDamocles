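; RuleWorld_BP is a game rule Blueprint that spawns waves of Alpha and Beta AI creeps at two target points.
; The LoopSpawn event increments a counter, waits briefly, spawns one creep of each type, then calls itself until the counter reaches MaxLoopSpawn.
; Nothing in this graph starts the loop: BeginPlay is empty and a delayed entry into the loop is left disconnected.
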(event Custom|LoopSpawn
  (Variables|Default|SetLoopSpawnCount (+ (Variables|Default|GetLoopSpawnCount) 1))
  (Utilities|FlowControl|Delay 0.5)
  (AI|SpawnAIFromClass "/Game/MOBAFight/Blueprint/AllActorInGame/CreepSystem/Creep_Alpha_BP.Creep_Alpha_BP_C" 0 (Transformation|GetActorLocation (Variables|Default|GetTargetPoint1)) "0, 0, 0" false 0)
  (AI|SpawnAIFromClass "/Game/MOBAFight/Blueprint/AllActorInGame/CreepSystem/Creep_Beta_BP.Creep_Beta_BP_C" 0 (Transformation|GetActorLocation (Variables|Default|GetTargetPoint2)) "0, 0, 0" false 0)
  (if (!= (Variables|Default|GetLoopSpawnCount) (Variables|Default|GetMaxLoopSpawn))
    (CallFunction|LoopSpawn)))

(event Collision|EventActorBeginOverlap
  (params (OtherActor :type Actor%20Object%20Reference)))

(event EventTick
  (params (DeltaSeconds :type Float%20%28single-precision%29)))

(event EventBeginPlay)

(fn ConstructionScript)